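; Superliminal-style forced-perspective puzzle for VR that hides a target actor and paints its image onto surrounding meshes.
; Scene captures of the target and depth-sorted surfaces feed M_Projection decals, built after BeginPlay or on demand.
; Entering the capsule eases the pawn to the capture point and shows look markers.
; Holding the matching view for about a second releases the real actor, restores the VR origin and destroys the projection.
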(event `Project`
  (bind _projection_target (`self.Projection Target`))
  (`self.Project Item` :!label _label)
  (`self.SetActorHiddenInGame` _projection_target true)
  (`self.SetActorEnableCollision` _projection_target false))

(event `self.ReceiveBeginPlay`
  (`KismetSystemLibrary.Delay` 1.0) ; Delay to Capture all Post processing
  (if (not (`self.On demand projection`))
    (goto _label)))

(event `self.ReceiveTick`
  (params (DeltaSeconds :type "Float (single-precision)"))
  ;[1 1 1] Tick Event
  (`self.Draw Line`)
  ;;[1 1 1] Center the player to the projection
  (`self.Player Near Position`)
  ;;[1 1 1] Check if player is in proper Position
  (if (`self.is Player in Position`)
    (`KismetSystemLibrary.Delay` 1.0)
    ;;[1 1 1] Check Player Position again
    (if (`self.is Player in Position`)
      (`self.Release the Actor`))))

(event `self.Capsule.OnComponentBeginOverlap`
  (params (OverlappedComponent :type "PrimitiveComponent Object Reference") (OtherActor :type "Actor Object Reference") (OtherComp :type "PrimitiveComponent Object Reference") (OtherBodyIndex :type Integer) (bFromSweep :type Boolean) (SweepResult :type "HitResult Structure (by ref)"))
  ;[1 1 1] Check if player near Projection and if so Enable Tick
  (bind _asvrpawn (cast `/Game/VRTemplate/Blueprints/VRPawn` OtherActor))
  (set `self.Player near` true)
  (set `self.Character` _asvrpawn)
  (`self.SetActorTickEnabled` true)
  (`ActorComponent.SetComponentTickEnabled` (`/Game/VRTemplate/Blueprints/BP_LookHere.BP_SmoothenCompoment` (`self.Camera Mark`)) true)
  (`self.SetActorHiddenInGame` (`self.Camera Mark`) false)
  (`self.SetActorHiddenInGame` (`self.Projection Mark`) false)
  (set `self.Original Transform` (`SceneComponent.GetRelativeTransform` (`/Game/VRTemplate/Blueprints/VRPawn.VROrigin` (`self.Character`)))))

(event `Destroy Actors`
  (`self.K2_DestroyActor` (`self.Camera Mark`))
  (`self.K2_DestroyActor` (`self.Projection Mark`))
  (`self.K2_DestroyActor` self))

(event `self.Capsule.OnComponentEndOverlap`
  (params (OverlappedComponent :type "PrimitiveComponent Object Reference") (OtherActor :type "Actor Object Reference") (OtherComp :type "PrimitiveComponent Object Reference") (OtherBodyIndex :type Integer))
  ;[1 1 1] Check if player near Projection and if so Enable Tick
)

(event `Release Player Lock`
  (bind _vrorigin (`/Game/VRTemplate/Blueprints/VRPawn.VROrigin` (`self.Character`)))
  ;[1 1 1] Disable/Enable movement (Not USed)
  (`self.Character`
    (:`then`
      (`/Engine/EditorBlueprintResources/StandardMacros.DoOnce` false :!label _label_2
        (:`Completed`
          (`self.SetActorHiddenInGame` (`self.Projection Mark`) true)
          (`self.SetActorHiddenInGame` (`self.Camera Mark`) true)
          (`self.SetActorHiddenInGame` self true)
          (`KismetSystemLibrary.Delay` 0.25)
          (bind (_direction _alpha) (`Timeline|Move Back Player` :!via `PlayFromStart`)
            (:`Update`
              (`SceneComponent.K2_SetRelativeTransform` _vrorigin (`KismetMathLibrary.TLerp` (`SceneComponent.GetRelativeTransform` _vrorigin) (`self.Original Transform`) _alpha) false true))
            (:`Finished`
              (`self.Destroy Actors`))))))
    (:`else`
      (goto _label_2 :!via `Reset`))))

(event `Disable Char Movement`
  ;[1 1 1] Disable/Enable movement (Not USed)
  (bind _character (`self.Character`)
    (:`then`
      (`CharacterMovementComponent.SetMovementMode` (`Character.CharacterMovement` _character) "MOVE_None" 0))
    (:`else`)))

(event `Enable Char Movement`
  ;[1 1 1] Disable/Enable movement (Not USed)
  (bind _character (`self.Character`)
    (:`then`
      (`CharacterMovementComponent.SetMovementMode` (`Character.CharacterMovement` _character) "MOVE_Walking" 0))
    (:`else`)))

(fn `Debug Arrow`
  (params (`Scene Component` :type "SceneComponent Object Reference") (LineColor :type "LinearColor Structure"))
  (bind _returnvalue (`SceneComponent.K2_GetComponentLocation` `Scene Component`))
  (`KismetSystemLibrary.DrawDebugLine` _returnvalue (+ _returnvalue (* (`KismetMathLibrary.GetForwardVector` (`SceneComponent.K2_GetComponentRotation` `Scene Component`)) 5000.0)) LineColor))

(fn `Draw Line`
  (bind _character (`self.Character`)
    (:`then`
      (bind _camera (`/Game/VRTemplate/Blueprints/VRPawn.Camera` _character))
      (bind _returnvalue (`SceneComponent.K2_GetComponentLocation` _camera))
      (bind (_outhit _returnvalue_2) (`KismetSystemLibrary.LineTraceSingle` _returnvalue (+ _returnvalue (* (`KismetMathLibrary.GetForwardVector` (`SceneComponent.K2_GetComponentRotation` _camera)) 2000.0)) "TraceTypeQuery1" false (`|MakeArray` _character :!type "Actor Object Reference")))
      (`self.SetActorHiddenInGame` (`self.Camera Mark`) (not _returnvalue_2))
      (`self.K2_SetActorLocation` (`self.Camera Mark`) (`.Location` (`GameplayStatics.BreakHitResult` _outhit)) false true))
    (:`else`)))

(fn `is Player in Position`
  (returns (Return :type Boolean))
  (bind _character (`self.Character`))
  (bind _returnvalue (and (== (- (`SceneComponent.K2_GetComponentLocation` (`self.SceneCaptureComponent2D`)) (`self.HMD Offset`)) (`SceneComponent.K2_GetComponentLocation` (`/Game/VRTemplate/Blueprints/VRPawn.VROrigin` _character)) :`ErrorTolerance` 2.0) (== (`SceneComponent.K2_GetComponentRotation` (`/Game/VRTemplate/Blueprints/VRPawn.Camera` _character)) (`SceneComponent.K2_GetComponentRotation` (`self.SceneCaptureComponent2D`)) :`ErrorTolerance` 3.0)))
  (`self.Character`
    (:`then`
      (`self.SetActorHiddenInGame` (`self.Projection Mark`) _returnvalue)
      (`self.SetActorHiddenInGame` (`self.Camera Mark`) _returnvalue)
      (return _returnvalue))
    (:`else`)))

(fn `Player Near Position`
  (bind _character (`self.Character`))
  (bind _character_2 (`self.Character`))
  (bind _vrorigin (`/Game/VRTemplate/Blueprints/VRPawn.VROrigin` _character_2))
  (if (`self.Player near`)
    (bind _character_3 (`self.Character`)
      (:`then`
        (`self.K2_SetActorLocation` _character (`KismetMathLibrary.VInterpTo` (`self.K2_GetActorLocation` _character) (`self.K2_GetActorLocation`) (`GameplayStatics.GetWorldDeltaSeconds`) 5.0) false false)
        (bind _output_get (set `self.HMD Offset` (`SceneComponent.RelativeLocation` (`/Game/VRTemplate/Blueprints/VRPawn.Camera` _character_2))))
        (`SceneComponent.K2_SetWorldLocation` _vrorigin (`KismetMathLibrary.VInterpTo` (`SceneComponent.K2_GetComponentLocation` _vrorigin) (- (`SceneComponent.K2_GetComponentLocation` (`self.SceneCaptureComponent2D`)) _output_get) (`GameplayStatics.GetWorldDeltaSeconds`) 5.0) false false)
        (return))
      (:`else`))))

(fn `Project Item`
  (bind _scenecapturecomponent2d (`self.SceneCaptureComponent2D`))
  (bind _scenecapturecomponent2dmask (`self.SceneCaptureComponent2DMask`))
  (`SceneComponent.K2_SetWorldRotation` (`self.SceneCaptureComponent2D`) (`KismetMathLibrary.FindLookAtRotation` (`SceneComponent.K2_GetComponentLocation` (`self.SceneCaptureComponent2D`)) (`self.K2_GetActorLocation` (`self.Projection Target`))) false false)
  (`SceneComponent.K2_SetWorldRotation` (`self.SceneCaptureComponent2DMask`) (`KismetMathLibrary.FindLookAtRotation` (`SceneComponent.K2_GetComponentLocation` (`self.SceneCaptureComponent2D`)) (`self.K2_GetActorLocation` (`self.Projection Target`))) false false)
  (`KismetArrayLibrary.Array_Add` (`SceneCaptureComponent.ShowOnlyActors` (`self.SceneCaptureComponent2D`)) (`self.Projection Target`))
  (`KismetArrayLibrary.Array_Add` (`SceneCaptureComponent.ShowOnlyActors` (`self.SceneCaptureComponent2DMask`)) (`self.Projection Target`))
  (`|ExecutionSequence`
    (:`then_0`
      (bind _returnvalue (`KismetRenderingLibrary.CreateRenderTarget2D` 2048 2048))
      (set `SceneCaptureComponent2D.TextureTarget` _returnvalue _scenecapturecomponent2d)
      (`SceneCaptureComponent2D.CaptureScene` _scenecapturecomponent2d)
      (set `Texture.CompressionQuality` "TCQ_Highest" _returnvalue))
    (:`then_1`
      (bind _returnvalue_2 (`KismetRenderingLibrary.CreateRenderTarget2D` 2048 2048))
      (set `SceneCaptureComponent2D.TextureTarget` _returnvalue_2 _scenecapturecomponent2dmask)
      (`SceneCaptureComponent2D.CaptureScene` _scenecapturecomponent2dmask))
    (:`then_2`
      (`self.Spawn Look Widget`))
    (:`then_3`
      (`self.Sort by Distance`))
    (:`then_4`
      (`self.Projection Trace`))
    (:`then_5`
      (`self.On Projection Creation`))))

(fn `Projection Trace`
  (locals (`Ignore Actors` :type "Array of Actor Object Reference") (`Current Target` :type "Actor Object Reference") (`Show Only` :type "Array of Actor Object Reference") (Decal :type "DecalComponent Object Reference") (`Transform Location` :type "Vector Structure" :default (0.0 0.0 0.0)) (`Local Location` :type "Vector Structure" :default (0.0 0.0 0.0)) (`Local Rotation` :type "Rotator Structure"))
  (bind (_start_location _end_location _scale _rotation) (`self.Trace Input`))
  (bind (_start_location_2 _end_location_2 _scale_2 _rotation_2) (`self.Trace Input`))
  (bind _decal (`local.Decal`))
  (`/Engine/EditorBlueprintResources/StandardMacros.IsValid` _decal
    (:`Is Valid`
      (`ActorComponent.K2_DestroyComponent` _decal)
      (`ActorComponent.K2_DestroyComponent` (`self.Scene Capture Depth`)))
    (:`Is Not Valid`
      _))
  (bind _outhits (`KismetSystemLibrary.BoxTraceMulti` _start_location _end_location _scale _rotation "TraceTypeQuery1" false (`self.Project On To`)))
  (for _array_element _outhits
    (`KismetArrayLibrary.Array_Add` (`local.Ignore Actors`) (`.HitActor` (`GameplayStatics.BreakHitResult` _array_element))))
  (for _array_element_2 (`self.Project On To`)
    (set `local.Current Target` _array_element_2)
    (bind _outhit (`KismetSystemLibrary.BoxTraceSingle` _start_location_2 _end_location_2 _scale_2 _rotation_2 "TraceTypeQuery1" false (`local.Ignore Actors`)))
    (`|ExecutionSequence`
      (:`then_0`
        (bind (_bblockinghit _binitialoverlap _time _distance _location _impactpoint _normal _impactnormal _physmat _hitactor _hitcomponent _hitbonename _bonename _hititem _elementindex _faceindex _tracestart _traceend) (`GameplayStatics.BreakHitResult` _outhit))
        (bind _asstatic_mesh_component (cast `StaticMeshComponent` _hitcomponent))
        (bind _returnvalue (`self.GetTransform` (`ActorComponent.GetOwner` _asstatic_mesh_component)))
        (bind (_min _max) (`StaticMeshComponent.GetLocalBounds` _asstatic_mesh_component))
        (set `local.Local Location` (+ (* (`KismetMathLibrary.Normal` (- _tracestart _traceend)) 5.1) (/ (+ (`KismetMathLibrary.TransformLocation` _returnvalue _min) (`KismetMathLibrary.TransformLocation` _returnvalue _max)) 2.0)))
        (set `local.Local Rotation` (`SceneComponent.K2_GetComponentRotation` _asstatic_mesh_component))
        (bind _returnvalue_2 (`AddComponent|NODE_AddDecalComponent-0` :`bManualAttachment` true :`RelativeTransform` (`KismetMathLibrary.MakeTransform` (`local.Local Location`) (`local.Local Rotation`))))
        (bind _output_get (set `local.Decal` _returnvalue_2))
        (`SceneComponent.SetWorldScale3D` _output_get (+ (* _max (`SceneComponent.K2_GetComponentScale` _asstatic_mesh_component)) 5.0))
        (bind _returnvalue_3 (`KismetRenderingLibrary.CreateRenderTarget2D` 1024 1024))
        (bind _returnvalue_4 (`AddComponent|NODE_AddSceneCaptureComponent2D-0` :`RelativeTransform` (`SceneComponent.GetRelativeTransform` (`self.SceneCaptureComponent2D`))))
        (bind _output_get_2 (set `self.Scene Capture Depth` _returnvalue_4))
        (set `SceneCaptureComponent2D.PostProcessSettings` (`SceneCaptureComponent2D.PostProcessSettings` (`self.SceneCaptureComponent2D`)) _output_get_2)
        (bind _output_get_3 (set `SceneCaptureComponent2D.TextureTarget` _returnvalue_3 _returnvalue_4))
        (`KismetArrayLibrary.Array_Append` (`SceneCaptureComponent.ShowOnlyActors` _returnvalue_4) (`local.Show Only`))
        (`SceneCaptureComponent2D.CaptureScene` _returnvalue_4)
        (bind _returnvalue_5 (`KismetMaterialLibrary.CreateDynamicMaterialInstance` "/Game/Superliminal/Projection/Material/M_Projection.M_Projection"))
        (`DecalComponent.SetDecalMaterial` (`local.Decal`) _returnvalue_5)
        (`self.Update Material Properties` _returnvalue_5 _output_get_3))
      (:`then_1`
        (`KismetArrayLibrary.Array_Add` (`local.Show Only`) (`local.Current Target`))
        (`KismetArrayLibrary.Array_Add` (`local.Ignore Actors`) (`local.Current Target`))))))

(fn `Release the Actor`
  (bind _projection_target (`self.Projection Target`))
  (`self.On Object Release`)
  (`self.SetActorHiddenInGame` _projection_target false)
  (`self.SetActorEnableCollision` _projection_target true)
  (bind _actor (message `/Game/Superliminal/Character/Blueprints/Interactions/BPI_Prop_Object.Get Prop Actor` (`self.Projection Target`)))
  (`/Engine/EditorBlueprintResources/StandardMacros.IsValid` _actor
    (:`Is Valid`
      (set `/Game/Superliminal/Prop/BP_MasterProp.IsLocked` false _actor)
      (`PrimitiveComponent.SetSimulatePhysics` (`/Game/Superliminal/Prop/BP_MasterProp.Prop` _actor) true)
      (`self.Enable Char Movement`)
      (`self.Release Player Lock`))
    (:`Is Not Valid`
      (`self.Enable Char Movement`)
      (`self.Release Player Lock`)))
  (`self.SetActorTickEnabled` false))

(fn `Sort by Distance`
  (locals (`Local index 1` :type Integer) (`Local Actor 1` :type "Actor Object Reference") (`Local index 2` :type Integer) (`Local Actor 2` :type "Actor Object Reference"))
  (for (_array_element _array_index) (`self.Project On To`)
    (set `local.Local index 1` _array_index)
    (set `local.Local Actor 1` _array_element)
    (for _index (range (`local.Local index 1`) (+ (`KismetArrayLibrary.Array_LastIndex` (`self.Project On To`)) 1))
      (bind _output_get (set `local.Local index 2` _index))
      (set `local.Local Actor 2` (`|GetArrayItem` (`self.Project On To`) _output_get))
      (if (< (`self.GetDistanceTo` (`local.Local Actor 2`)) (`self.GetDistanceTo` (`local.Local Actor 1`)))
        (`KismetArrayLibrary.Array_Swap` (`self.Project On To`) (`local.Local index 1`) (`local.Local index 2`))))))

(fn `Spawn Look Widget`
  (bind _returnvalue_location (`KismetMathLibrary.BreakTransform` (`self.GetTransform` (`self.Projection Target`))))
  (`|ExecutionSequence`
    (:`then_0`
      (bind _returnvalue (`|SpawnActorFromClass` "/Game/VRTemplate/Blueprints/BP_LookHere.BP_LookHere_C" (`KismetMathLibrary.MakeTransform` _returnvalue_location (`SceneComponent.K2_GetComponentRotation` (`self.SceneCaptureComponent2D`))) "AlwaysSpawn" "MultiplyWithRoot" null null))
      (set `self.Projection Mark` _returnvalue))
    (:`then_1`
      (bind _returnvalue_2 (`|SpawnActorFromClass` "/Game/VRTemplate/Blueprints/BP_LookHere.BP_LookHere_C" (`self.GetTransform`) "AlwaysSpawn" "MultiplyWithRoot" null null))
      (set `self.Camera Mark` _returnvalue_2)
      (bind _asvrpawn (cast `/Game/VRTemplate/Blueprints/VRPawn` (`GameplayStatics.GetPlayerPawn` 0)))
      (set `/Game/VRTemplate/Blueprints/BP_SmoothenCompoment.Follow Target` (`/Game/VRTemplate/Blueprints/VRPawn.Camera` _asvrpawn) (`/Game/VRTemplate/Blueprints/BP_LookHere.BP_SmoothenCompoment` (`self.Camera Mark`)))
      (bind _aswb_point (cast `/Game/VRTemplate/Blueprints/WB_Point` (`WidgetComponent.GetUserWidgetObject` (`/Game/VRTemplate/Blueprints/BP_LookHere.Widget` (`self.Camera Mark`)))))
      (`/Game/VRTemplate/Blueprints/WB_Point.Player Crosshair` _aswb_point))
    (:`then_2`
      (`self.SetActorHiddenInGame` (`self.Projection Mark`) true)
      (`self.SetActorHiddenInGame` (`self.Camera Mark`) true))))

(fn `Trace Input`
  (returns (`Start Location` :type "Vector Structure") (`End Location` :type "Vector Structure") (Scale :type "Vector Structure") (Rotation :type "Rotator Structure"))
  (bind _returnvalue (`SceneComponent.K2_GetComponentLocation` (`self.SceneCaptureComponent2D`)))
  (bind _prop (message `/Game/Superliminal/Character/Blueprints/Interactions/BPI_Prop_Object.Get Prop Mesh` (`self.Projection Target`)))
  (return _returnvalue (+ _returnvalue (* (`SceneComponent.GetForwardVector` (`self.SceneCaptureComponent2D`)) 5000.0)) (`KismetMathLibrary.SelectVector` (`.BoxExtent` (`KismetSystemLibrary.GetComponentBounds` _prop)) (100.0 100.0 100.0) (`KismetSystemLibrary.IsValid` _prop)) (`SceneComponent.K2_GetComponentRotation` (`self.SceneCaptureComponent2D`))))

(fn `Unique Items`
  (locals (`Temp Array` :type "Array of Actor Object Reference"))
  (bind _temp_array (`local.Temp Array`))
  (for _array_element (`self.Project On To`)
    (`KismetArrayLibrary.Array_AddUnique` (`local.Temp Array`) _array_element))
  (set `self.Project On To` _temp_array)
  (`KismetArrayLibrary.Array_Clear` _temp_array))

(fn `Update Material Properties`
  (params (Mat :type "MaterialInstanceDynamic Object Reference") (Texture :type "TextureRenderTarget2D Object Reference"))
  (`MaterialInstanceDynamic.SetVectorParameterValue` Mat "Location" (`KismetMathLibrary.Conv_VectorToLinearColor` (`SceneComponent.K2_GetComponentLocation` (`self.SceneCaptureComponent2D`))))
  (`MaterialInstanceDynamic.SetVectorParameterValue` Mat "Right Vector" (`KismetMathLibrary.Conv_VectorToLinearColor` (`SceneComponent.GetRightVector` (`self.SceneCaptureComponent2D`))))
  (`MaterialInstanceDynamic.SetVectorParameterValue` Mat "Up Vector" (`KismetMathLibrary.Conv_VectorToLinearColor` (`SceneComponent.GetUpVector` (`self.SceneCaptureComponent2D`))))
  (`MaterialInstanceDynamic.SetVectorParameterValue` Mat "Forward Vector" (`KismetMathLibrary.Conv_VectorToLinearColor` (`SceneComponent.GetForwardVector` (`self.SceneCaptureComponent2D`))))
  (`MaterialInstanceDynamic.SetScalarParameterValue` Mat "Fov" (`SceneCaptureComponent2D.FOVAngle` (`self.SceneCaptureComponent2D`)))
  (`MaterialInstanceDynamic.SetTextureParameterValue` Mat "Projected Texture" (`SceneCaptureComponent2D.TextureTarget` (`self.SceneCaptureComponent2D`)))
  (`MaterialInstanceDynamic.SetTextureParameterValue` Mat "Projected Mask" Texture)
  (`MaterialInstanceDynamic.SetTextureParameterValue` Mat "Actor Mask" (`SceneCaptureComponent2D.TextureTarget` (`self.SceneCaptureComponent2DMask`))))

(fn `UserConstructionScript`
  (bind _retro_post_processing_volume (`self.Retro Post Processing Volume`))
  (bind _settings (`PostProcessComponent.Settings` (`/Game/RetroShadersV4/RetroShader/BP_RetroPostProcess.PostProcess` _retro_post_processing_volume)))
  (set `PrimitiveComponent.bGenerateOverlapEvents` (`self.Should Generate Event`) (`self.Capsule`))
  (`self.Unique Items`)
  (`/Engine/EditorBlueprintResources/StandardMacros.IsValid` _retro_post_processing_volume
    (:`Is Valid`
      (set `SceneCaptureComponent2D.PostProcessSettings` _settings (`self.SceneCaptureComponent2DMask`))
      (set `SceneCaptureComponent2D.PostProcessSettings` _settings (`self.SceneCaptureComponent2D`)))))