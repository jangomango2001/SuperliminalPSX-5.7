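; BP_ResetButton is a button prop that triggers a reset when the player tries to pick it up.
; Its PickUp override skips the parent logic, calls CallReset, plays the press feedback and returns false.
; The feedback is a timeline that slides the Prop along relative X plus a 2D switch click.
; A separate ChangeMaterial event applies the Signed_paper material to the Prop and is not called within this file.
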(event `Change Material`
  (if (not false)
    (`PrimitiveComponent.SetMaterial` (`self.Prop`) 0 "/Game/PSX_Models/Materials/Signed_paper.Signed_paper")))

(event `Play Sound`
  (`GameplayStatics.PlaySound2D` "/Game/Superliminal/Audio/Switch_Click.Switch_Click" 0.5 1.0 0.0 null null))

(event `Play Button Animation`
  (bind (_direction _switch_position) (`Timeline|Timeline` :!via `PlayFromStart`)
    (:`Update`
      (`SceneComponent.K2_SetRelativeLocation` (`self.Prop`) (`KismetMathLibrary.MakeVector` _switch_position) false false))))

(fn `PickUp`
  (params (`Parent Comp` :type "SceneComponent Object Reference"))
  (returns (`Picked Up?` :type Boolean))
  (`self.Reset`)
  (`self.Play Button Animation`)
  (`self.Play Sound`)
  (return false))

(fn `UserConstructionScript`
  (`parent.UserConstructionScript`))