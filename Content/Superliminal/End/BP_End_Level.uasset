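; End-of-level trigger for a Superliminal-style game that fires when the VRPawn overlaps its box.
; It disables the pawn's input, stops its movement and undoes its size change by resizing with the inverse of LastSizeIn.
; Once only, it hands LevelToLoad to the game instance, starts the fade-in widget and saves newest and unlocked levels, leaving the direct level-stream load unwired.
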(event `self.Box.OnComponentBeginOverlap`
  (params (OverlappedComponent :type "PrimitiveComponent Object Reference") (OtherActor :type "Actor Object Reference") (OtherComp :type "PrimitiveComponent Object Reference") (OtherBodyIndex :type Integer) (bFromSweep :type Boolean) (SweepResult :type "HitResult Structure (by ref)"))
  (bind _asvrpawn (cast `/Game/VRTemplate/Blueprints/VRPawn` OtherActor))
  (bind _my_game_instance_ref (message `/Game/Superliminal/BPI_GameInstance.Get Game instance` (`GameplayStatics.GetGameInstance`)))
  (`/Engine/EditorBlueprintResources/StandardMacros.IsValid` _my_game_instance_ref
    (:`Is Valid`
      (`/Engine/EditorBlueprintResources/StandardMacros.DoOnce` false :!label _label
        (:`Completed`
          (`self.DisableInput` _asvrpawn (cast `PlayerController` (`Pawn.GetController` _asvrpawn) :!pure true))
          (`MovementComponent.StopMovementImmediately` (`Character.CharacterMovement` _asvrpawn))
          (`/Game/VRTemplate/Blueprints/VRPawn.Resize Player` _asvrpawn (/ 1.0 (`/Game/VRTemplate/Blueprints/VRPawn.Last Size In` _asvrpawn)))
          (set `/Game/Superliminal/MygameInstance.New Level Name` (`self.Level to Load`) _my_game_instance_ref)
          (`/Game/Superliminal/MygameInstance.Fade In Widget` _my_game_instance_ref)
          (`/Game/Superliminal/MygameInstance.Save Newest Level` _my_game_instance_ref)
          (`/Game/Superliminal/MygameInstance.Save unlocked Levels` _my_game_instance_ref))))
    (:`Is Not Valid`
      (goto _label :!via `Reset`))))

(fn `UserConstructionScript`)