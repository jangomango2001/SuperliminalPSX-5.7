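; BP_PortalNew is a holdable Superliminal-style portal that teleports the VR player to its LinkingPortal and resizes them by the two portals' scale ratio.
; Overlapping from the front while neither holding nor held arms a Tick check, using a velocity-predicted dot product to detect crossing.
; Teleporting remaps location, rotation and velocity through the linked BackFace transform, briefly disabling collision on both portals.
; While held, its rotation resets every tick.
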(event `self.ReceiveBeginPlay`
  (bind _asvrpawn (cast `/Game/VRTemplate/Blueprints/VRPawn` (`GameplayStatics.GetPlayerPawn` 0) :!label _label)
    (:`then`
      (set `self.Character Ref` _asvrpawn))
    (:`CastFailed`
      (`KismetSystemLibrary.Delay` 0.2)
      (goto _label))))

(event `self.ReceiveTick`
  (params (DeltaSeconds :type "Float (single-precision)"))
  (bind _returnvalue (`GameplayStatics.GetPlayerPawn` 0))
  (`|ExecutionSequence`
    (:`then_0`
      (if (`self.IsHeld`)
        (`self.Reset Rotation`)))
    (:`then_1`
      (if (`self.Start Overlap`)
        (if (and (not (`self.IsHeld`)) (>= (`KismetMathLibrary.Dot_VectorVector` (`SceneComponent.GetForwardVector` (`self.Prop`)) (`KismetMathLibrary.Normal` (- (`SceneComponent.K2_GetComponentLocation` (`self.Prop`)) (+ (`self.K2_GetActorLocation` _returnvalue) (* (`self.GetVelocity` _returnvalue) (`GameplayStatics.GetWorldDeltaSeconds`)))))) 0.0))
          (`self.Teleport Player`))))))

(event `self.Drop Prop.OnComponentBeginOverlap`
  (params (OverlappedComponent :type "PrimitiveComponent Object Reference") (OtherActor :type "Actor Object Reference") (OtherComp :type "PrimitiveComponent Object Reference") (OtherBodyIndex :type Integer) (bFromSweep :type Boolean) (SweepResult :type "HitResult Structure (by ref)"))
  (bind _returnvalue (`GameplayStatics.GetPlayerPawn` 0))
  (if (not (`self.IsHeld`))
    (if (== OtherActor _returnvalue)
      (if (not (`/Game/VRTemplate/Blueprints/VRPawn.IsHolding?` (cast `/Game/VRTemplate/Blueprints/VRPawn` _returnvalue :!pure true)))
        (if (`self.Is Player in Front`)
          (set `self.Start Overlap` true))))))

(event `self.Drop Prop.OnComponentEndOverlap`
  (params (OverlappedComponent :type "PrimitiveComponent Object Reference") (OtherActor :type "Actor Object Reference") (OtherComp :type "PrimitiveComponent Object Reference") (OtherBodyIndex :type Integer))
  (if (not (`self.IsHeld`))
    (if (== OtherActor (`GameplayStatics.GetPlayerPawn` 0))
      (set `self.Start Overlap` false))))

(event `Enable Back Collision`
  (`KismetSystemLibrary.Delay` 1.25)
  (`self.Enable/Disable Mesh Collision` true))

(fn `Enable Disable Backface Collision`
  (params (`Is facing portal` :type Boolean))
  (`PrimitiveComponent.SetCollisionEnabled` (`self.PortalPlane`) (select `bool` `Is facing portal` :`false` "QueryAndPhysics" :`true` "NoCollision" :!type "ECollisionEnabled Enum")))

(fn `Enable/Disable Mesh Collision`
  (params (`Enable Collision` :type Boolean))
  (bind _prop (`self.Prop`))
  (if `Enable Collision`
    (`PrimitiveComponent.SetCollisionEnabled` _prop "QueryAndPhysics")
    (`PrimitiveComponent.SetCollisionEnabled` (`/Game/Superliminal/Prop/BP_MasterProp.Prop` (`self.Linking Portal`)) "QueryAndPhysics")
    (`self.SetActorEnableCollision` (`self.Linking Portal`) true)
    (else
      (`PrimitiveComponent.SetSimulatePhysics` (`/Game/Superliminal/Prop/BP_MasterProp.Prop` (`self.Linking Portal`)) false)
      (`PrimitiveComponent.SetSimulatePhysics` _prop false)
      (`PrimitiveComponent.SetCollisionEnabled` _prop "NoCollision")
      (`PrimitiveComponent.SetCollisionEnabled` (`/Game/Superliminal/Prop/BP_MasterProp.Prop` (`self.Linking Portal`)) "NoCollision")
      (`self.SetActorEnableCollision` (`self.Linking Portal`) false))))

(fn `Is Player in Front`
  (returns (Return :type Boolean))
  (bind _returnvalue (>= (`KismetMathLibrary.Dot_VectorVector` (`SceneComponent.GetForwardVector` (`self.Prop`)) (`KismetMathLibrary.Normal` (- (`self.K2_GetActorLocation` (`GameplayStatics.GetPlayerPawn` 0)) (`SceneComponent.K2_GetComponentLocation` (`self.Prop`))))) 0.0))
  (`self.Enable Disable Backface Collision` _returnvalue)
  (return _returnvalue))

(fn `Teleport Player`
  (locals (`Player Velocity` :type "Vector Structure") (Location :type "Vector Structure") (Rotation :type "Rotator Structure" :default (struct)))
  (bind _returnvalue_x (`KismetMathLibrary.BreakVector` (`SceneComponent.K2_GetComponentScale` (`self.Prop`))))
  (bind (_returnvalue_x_2 _returnvalue_y _returnvalue_z) (`KismetMathLibrary.BreakVector` (`SceneComponent.K2_GetComponentScale` (`/Game/Superliminal/Prop/BP_MasterProp.Prop` (`self.Linking Portal`)))))
  (`self.Character Ref`
    (:`then`
      (set `local.Player Velocity` (`KismetMathLibrary.TransformDirection` (`SceneComponent.K2_GetComponentToWorld` (`/Game/Superliminal/Portal/BP_PortalNew.BackFace` (`self.Linking Portal`))) (`KismetMathLibrary.InverseTransformDirection` (`SceneComponent.K2_GetComponentToWorld` (`self.Prop`)) (`self.GetVelocity` (`self.Character Ref`)))))
      (set `local.Location` (`KismetMathLibrary.TransformLocation` (`SceneComponent.K2_GetComponentToWorld` (`/Game/Superliminal/Portal/BP_PortalNew.BackFace` (`self.Linking Portal`))) (`KismetMathLibrary.InverseTransformLocation` (`SceneComponent.K2_GetComponentToWorld` (`self.Prop`)) (`self.K2_GetActorLocation` (`self.Character Ref`)))))
      (set `local.Rotation` (`KismetMathLibrary.TransformRotation` (`SceneComponent.K2_GetComponentToWorld` (`/Game/Superliminal/Portal/BP_PortalNew.BackFace` (`self.Linking Portal`))) (`KismetMathLibrary.InverseTransformRotation` (`SceneComponent.K2_GetComponentToWorld` (`self.Prop`)) (`self.K2_GetActorRotation` (`self.Character Ref`)))))
      (`self.Enable/Disable Mesh Collision` false)
      (`/Game/VRTemplate/Blueprints/VRPawn.Resize Player` (`self.Character Ref`) (/ _returnvalue_z _returnvalue_x))
      (`self.K2_SetActorLocationAndRotation` (`self.Character Ref`) (`local.Location`) (`local.Rotation`) false true)
      (set `MovementComponent.Velocity` (`local.Player Velocity`) (`Character.CharacterMovement` (`self.Character Ref`)))
      (`self.Enable Back Collision`))
    (:`else`)))

(fn `UserConstructionScript`)