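; Portal capture actor variant that permanently stops ticking once the player pawn overlaps it.
; When ReverseToggle is set, a looping timer enables tick only while the player is within a fixed distance of ViewingPortal.
; On player overlap it disables tick and invalidates that timer, and the empty leave event never restores it.
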(event `Enable Tick`
  (`self.SetActorTickEnabled` (not (>= (`KismetMathLibrary.Vector_Distance` (`self.K2_GetActorLocation` (`self.ViewingPortal`)) (`self.K2_GetActorLocation` (`GameplayStatics.GetPlayerPawn` 0))) 6000.0))))

(event `self.ReceiveBeginPlay`
  (`parent.ReceiveBeginPlay`)
  (if (`self.Reverse Toggle`)
    (bind _returnvalue (`KismetSystemLibrary.K2_SetTimerDelegate` (delegate `Enable Tick`) 1.0 true))
    (set `self.Timer` _returnvalue)))

(event `self.On Actor Overlap`
  (params (OverlappedActor :type "Actor Object Reference") (OtherActor :type "Actor Object Reference"))
  (bind _timer (`self.Timer`))
  (if (== OtherActor (`GameplayStatics.GetPlayerPawn` 0))
    (`self.SetActorTickEnabled` false)
    (if (`KismetSystemLibrary.K2_IsValidTimerHandle` (`self.Timer`))
      (`KismetSystemLibrary.K2_PauseTimerHandle` _timer)
      (`KismetSystemLibrary.K2_InvalidateTimerHandle` _timer))))

(event `self.On Actor Leave`
  (params (OverlappedActor :type "Actor Object Reference") (OtherActor :type "Actor Object Reference")))

(fn `UserConstructionScript`
  (`parent.UserConstructionScript`))